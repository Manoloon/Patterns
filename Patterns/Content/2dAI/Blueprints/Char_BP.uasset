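; Char_BP is an AI character that detects other characters ahead and can fire projectiles.
; In one PatronAI mode, Tick line-traces along Arrow1, with WorldDynamic hits blocking detection; a new Pawn hit changes Estado and, if Char_BP, gets the friendly material.
; StartShoot spawns Proyectil_BP at the arrow; StopShoot resets Estado.
; Construction caches waypoint locations and applies the material; data-table and widget logic is disconnected.
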(event Custom|Start%20Shoot
  (Game|SpawnActorfromClass "/Game/2dAI/Blueprints/Proyectil_BP.Proyectil_BP_C" (Math|Transform|MakeTransform (Transformation|GetWorldLocation (Variables|Default|GetArrow1)) "0, 0, 0" "0.200000,0.200000,0.200000") "AdjustIfPossibleButAlwaysSpawn" 0 0))

(event Custom|Stop%20Shoot
  (Variables|Default|SetEstado "NewEnumerator0"))

(event EventBeginPlay)

(event EventTick
  (params (DeltaSeconds :type Float%20%28single-precision%29))
  (if (Utilities|Enum|Equal(Enum) (Variables|Default|GetPatronAI) "NewEnumerator1")
    (CallFunction|CheckEnemyAhead)))

(fn ConstructionScript
  (Variables|Default|SetLoc_A (Transformation|GetActorLocation (Variables|Default|GetWayPoint_A)))
  (Variables|Default|SetLoc_B (Transformation|GetActorLocation (Variables|Default|GetWaypoint_B)))
  (Rendering|Material|SetMaterial (Variables|Character|GetMesh) 0 (Variables|Default|GetMaterial)))

(fn CheckEnemyAhead
  (bind _returnvalue (Transformation|GetActorLocation))
  (bind _arrow1 (Variables|Default|GetArrow1))
  (bind _returnvalue_2 (Math|Vector|GetForwardVector _arrow1))
  (bind _returnvalue_3 (* _returnvalue_2 1e+03))
  (bind _returnvalue_4 (+ _returnvalue _returnvalue_3))
  (bind (_outhit _returnvalue_5) (Collision|LineTraceForObjects _returnvalue _returnvalue_4 (Utilities|Array|MakeArray "ObjectTypeQuery2") false 0 "ForOneFrame" true "(R=1.000000,G=0.000000,B=0.000000,A=1.000000)" "(R=0.000000,G=0.135954,B=1.000000,A=1.000000)"))
  (if _returnvalue_5
    (Development|PrintString "hit wall")
    (Variables|Default|SetEstado "NewEnumerator0")
    (else
      (bind (_outhit_2 _returnvalue_6) (Collision|LineTraceForObjects _returnvalue _returnvalue_4 (Utilities|Array|MakeArray "ObjectTypeQuery3") false 0 "ForOneFrame"))
      (if _returnvalue_6
        (if (!= (.HitActor (Collision|BreakHitResult _outhit_2)) (Variables|Default|GetEnemyCharacter))
          (bind _output_get (Variables|Default|SetEnemyCharacter (.HitActor (Collision|BreakHitResult _outhit_2))))
          (bind _aschar_bp (Utilities|Casting|CastToChar_BP _output_get))
          (Rendering|Material|SetMaterial (Variables|/Script/Engine.Character|GetMesh _aschar_bp) 0 "/Game/2dAI/Materials/CharFriendly_MT_Inst.CharFriendly_MT_Inst")
          (Variables|Default|SetEstado "NewEnumerator1"))
        (else
          (Variables|Default|SetEnemyCharacter 0)
          (Variables|Default|SetEstado "NewEnumerator0"))))))